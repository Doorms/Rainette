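; BP_FHat1 is a pickup, by its name a hat, that follows the player once its trigger box is overlapped.
; BeginPlay caches the BP_Player reference, and the first overlap by any actor sets an Attach flag and destroys the box.
; While the flag is set, Tick copies the world location and rotation of the player's Scene component to the root, rather than using component attachment.
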(event OnComponentBeginOverlap(Box)
  (params (OverlappedComponent :type Primitive%20Component%20Object%20Reference) (OtherActor :type Actor%20Object%20Reference) (OtherComp :type Primitive%20Component%20Object%20Reference) (OtherBodyIndex :type Integer) (bFromSweep :type Boolean) (SweepResult :type Hit%20Result%20Structure%20%28by%20ref%29))
  (Variables|Default|SetAttach? true)
  (Components|DestroyComponent (Variables|Default|GetBox)))

(event EventTick
  (params (DeltaSeconds :type Float%20%28single-precision%29))
  (bind _bp_playerref (Variables|Default|GetBP_PlayerRef))
  (bind _scene (Variables|/Game/Blueprints/BP_Player.BP_Player_C|GetScene _bp_playerref))
  (if (Variables|Default|GetAttach?)
    (Transformation|SetWorldLocationAndRotation (Variables|Default|GetDefaultSceneRoot) (Transformation|GetWorldLocation _scene) (Transformation|GetWorldRotation _scene) false false)))

(event EventBeginPlay
  (bind _asbp_player (Utilities|Casting|CastToBP_Player (Game|GetPlayerCharacter 0)))
  (Variables|Default|SetBP_PlayerRef _asbp_player))

(fn ConstructionScript)